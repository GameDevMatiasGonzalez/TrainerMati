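; BP_Soda is a soda bottle actor that takes on one of four random effect types when it spawns.
; On BeginPlay a random roll sets the Efecto enum with weighted odds, rarest to most common, and swaps the BottleWater material to match.
; The capsule overlap event is empty and the DestroyActor call is unwired, so the file applies no effect and has no pickup behavior.
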(event `self.ReceiveBeginPlay`
  (bind _output_get (set `self.Numero` (`KismetMathLibrary.RandomIntegerInRange` 0 99)))
  (if (`KismetMathLibrary.InRange_IntInt` _output_get 0 9)
    (set `self.Efecto` "NewEnumerator0")
    (`PrimitiveComponent.SetMaterial` (`self.Bottle_Water`) 0 "/Game/Soda/M_Soda.M_Soda")
    (elif (`KismetMathLibrary.InRange_IntInt` _output_get 10 29)
      (set `self.Efecto` "NewEnumerator1")
      (`PrimitiveComponent.SetMaterial` (`self.Bottle_Water`) 0 "/Game/Soda/M_Soda_3.M_Soda_3")
      (elif (`KismetMathLibrary.InRange_IntInt` _output_get 30 59)
        (set `self.Efecto` "NewEnumerator2")
        (`PrimitiveComponent.SetMaterial` (`self.Bottle_Water`) 0 "/Game/Soda/M_Soda_2.M_Soda_2")
        (elif (`KismetMathLibrary.InRange_IntInt` _output_get 60 99)
          (set `self.Efecto` "NewEnumerator3")
          (`PrimitiveComponent.SetMaterial` (`self.Bottle_Water`) 0 "/Game/Soda/M_Soda_4.M_Soda_4"))))))

(event `self.Capsule.OnComponentBeginOverlap`
  (params (OverlappedComponent :type "PrimitiveComponent Object Reference") (OtherActor :type "Actor Object Reference") (OtherComp :type "PrimitiveComponent Object Reference") (OtherBodyIndex :type Integer) (bFromSweep :type Boolean) (SweepResult :type "HitResult Structure (by ref)")))

(fn `UserConstructionScript`)